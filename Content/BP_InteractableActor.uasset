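; BP_InteractableActor is an actor that shows an interaction prompt when a qualifying actor enters its Box trigger.
; Overlapping actors are checked through CanInteractMessage; a match lazily creates and shows WB_Interact and enables input for player controller 0.
; Leaving the box removes the widget and disables input.
; Pressing Interact hides the prompt and only prints a debug string, with no further interaction logic.
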(event `self.Box.OnComponentBeginOverlap`
  (params (OverlappedComponent :type "PrimitiveComponent Object Reference") (OtherActor :type "Actor Object Reference") (OtherComp :type "PrimitiveComponent Object Reference") (OtherBodyIndex :type Integer) (bFromSweep :type Boolean) (SweepResult :type "HitResult Structure (by ref)"))
  (bind _binteract (message `/Game/BPI_Interact.CanInteract` OtherActor))
  (if _binteract
    (`self.WBInteract`
      (:`then`
        _)
      (:`else`
        (bind _returnvalue (`|CreateWidget` "/Game/UI/WB_Interact.WB_Interact_C"))
        (bind _output_get (set `self.WBInteract` _returnvalue))))
    (`UserWidget.AddToViewport` _output_get 0)
    (`self.EnableInput` (`GameplayStatics.GetPlayerController` 0))))

(event `self.Box.OnComponentEndOverlap`
  (params (OverlappedComponent :type "PrimitiveComponent Object Reference") (OtherActor :type "Actor Object Reference") (OtherComp :type "PrimitiveComponent Object Reference") (OtherBodyIndex :type Integer))
  (bind _binteract (message `/Game/BPI_Interact.CanInteract` OtherActor))
  (if _binteract
    (bind _wbinteract (`self.WBInteract`)
      (:`then`
        (if (`Widget.IsInViewport` _wbinteract)
          (`Widget.RemoveFromParent` (`self.WBInteract`))))
      (:`else`
        _))
    (`self.DisableInput` (`GameplayStatics.GetPlayerController` 0))))

(event `Key|E`
  (params (Key :type "Key Structure")))

(event `InputAction|Interact`
  (params (Key :type "Key Structure"))
  (:`Pressed`
    (bind _wbinteract (`self.WBInteract`)
      (:`then`
        (if (`Widget.IsInViewport` _wbinteract)
          (`Widget.RemoveFromParent` (`self.WBInteract`))))
      (:`else`
        _))
    (`KismetSystemLibrary.PrintString` "Player Interacting")))

(fn `UserConstructionScript`)