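; BP_MyPlayerController is a Blueprint player controller with no active logic, as its BeginPlay, Tick and construction script are empty.
; Disconnected node chains remain in the event graph and never run.
; They would call debug and test functions on the BP_Player inventory system, create a HUD widget, and display the player menu.
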(event `self.ReceiveBeginPlay`)

(event `InputAction|Interact`
  (params (Key :type "Key Structure")))

(event `Key|One`
  (params (Key :type "Key Structure")))

(fn `UserConstructionScript`)